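; BP_FarmTile is a farm plot actor that can be tilled, watered and planted, and shows the matching ground and crop meshes.
; Each action updates the TileState struct, then rebuilds graphics using dynamic alpha-clip materials.
; Plant meshes and textures come from a growth lookup on GI_ForgottenFrontier, keyed by plant name and growth stage.
; It also registers four directional snap targets, and a dev function steps through till, water, plant and grow.
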(event EventBeginPlay
  (Actions|InitRefs)
  (CallFunction|InitSnapTargets)
  (CallFunction|InitGraphics))

(event Collision|EventActorBeginOverlap
  (params (OtherActor :type Actor%20Object%20Reference)))

(event EventTick
  (params (DeltaSeconds :type Float%20%28single-precision%29)))

(fn ConstructionScript)

(fn InitSnapTargets
  (Utilities|Array|Add (Variables|Default|GetsnapTargets) (Variables|Default|GetWestSnap))
  (Utilities|Array|Add (Variables|Default|GetsnapTargets) (Variables|Default|GetEastSnap))
  (Utilities|Array|Add (Variables|Default|GetsnapTargets) (Variables|Default|GetNorthSnap))
  (Utilities|Array|Add (Variables|Default|GetsnapTargets) (Variables|Default|GetSouthSnap)))

(fn InitGraphics
  (CallFunction|InitGroundGraphics)
  (CallFunction|InitPlantGraphics))

(fn InitGroundGraphics
  (bind _tilestate (Variables|Default|GettileState))
  (bind _groundmesh (Variables|Default|GetGroundMesh))
  (bind _groundstate (Utilities|Struct|BreakSTR_FarmTileState _tilestate))
  (bind _returnvalue (Utilities|Enum|Equal(Enum) _groundstate "NewEnumerator1"))
  (if (or (Utilities|Enum|Equal(Enum) _groundstate "NewEnumerator0") _returnvalue)
    (if _returnvalue
      (Components|StaticMesh|SetStaticMesh _groundmesh "/Game/Maps/Environment/FarmTile/Meshes/FarmTileWatered.FarmTileWatered")
      (else
        (Components|StaticMesh|SetStaticMesh _groundmesh "/Game/Maps/Environment/FarmTile/Meshes/FarmTile.FarmTile")))
    (Rendering|SetVisibility (Variables|Default|GetGroundMesh) true false)
    (bind _returnvalue_2 (Rendering|Material|CreateDynamicMaterialInstance "/Game/Materials/AlphaClipTextured_MAT.AlphaClipTextured_MAT" "None" "None" :!class /Script/Engine.KismetMaterialLibrary))
    (bind _output_get (LocalVariables|SetdynaMat _returnvalue_2))
    (Rendering|Material|SetTextureParameterValue _output_get "Texture" "/Game/Maps/Environment/Ground/Textures/FullEnvTexture.FullEnvTexture")
    (Rendering|Material|SetMaterial (Variables|Default|GetGroundMesh) 0 (LocalVariables|GetdynaMat))))

(fn InitPlantGraphics
  (bind _tilestate (Variables|Default|GettileState))
  (bind (_stringvals _intvals) (Utilities|Struct|BreakSTR_FarmTileState _tilestate))
  (bind _value (Utilities|Map|Find _stringvals "PlantName"))
  (if (Utilities|Enum|Equal(Enum) _value "None")
    (Development|PrintString "No plant??")
    (else
      (Rendering|SetVisibility (Variables|Default|GetPlantMesh) true false)
      (bind (_outgrowthrate _meshesbystage _textures) (Default|LookupPlantGrowthInfo (Variables|KeyRefs|GetGI_REF) _value))
      (Components|StaticMesh|SetStaticMesh (Variables|Default|GetPlantMesh) (.Value (Utilities|Map|Find _meshesbystage (.Value (Utilities|Map|Find _intvals "GrowthStage")))))
      (bind _returnvalue (Rendering|Material|CreateDynamicMaterialInstance "/Game/Materials/AlphaClipTextured_MAT.AlphaClipTextured_MAT" "None" "None" :!class /Script/Engine.KismetMaterialLibrary))
      (bind _output_get (LocalVariables|SetdynaMat _returnvalue))
      (Rendering|Material|SetTextureParameterValue _output_get "Texture" (.Value (Utilities|Map|Find _textures "Texture")))
      (Rendering|Material|SetMaterial (Variables|Default|GetPlantMesh) 0 (LocalVariables|GetdynaMat)))))

(fn TillTile
  (if (Utilities|Enum|Equal(Enum) (.GroundState (Utilities|Struct|BreakSTR_FarmTileState (Variables|Default|GettileState))) "NewEnumerator2")
    (Utilities|Struct|SetmembersinSTR_FarmTileState (Variables|Default|GettileState) "NewEnumerator0")
    (CallFunction|InitGraphics)))

(fn WaterTile
  (if (Utilities|Enum|Equal(Enum) (Utilities|Struct|BreakSTR_FarmTileState (Variables|Default|GettileState)) "NewEnumerator0")
    (Utilities|Struct|SetmembersinSTR_FarmTileState (Variables|Default|GettileState) "NewEnumerator1")
    (CallFunction|InitGraphics)))

(fn PlantSeed
  (params (inSeedPlanted :type String))
  (bind _output_get (LocalVariables|SetseedPlanted inSeedPlanted))
  (Utilities|Map|Add (.StringVals (Utilities|Struct|BreakSTR_FarmTileState (Variables|Default|GettileState))) "PlantName" _output_get)
  (CallFunction|InitGraphics))

(fn InitRefs
  (bind _asgi_forgotten_frontier (Utilities|Casting|CastToGI_ForgottenFrontier (Game|GetGameInstance)))
  (Variables|KeyRefs|SetGI_REF _asgi_forgotten_frontier))

(fn [DEV]InteractwithTile
  (bind _tilestate (Variables|Default|GettileState))
  (bind _intvals (Utilities|Struct|BreakSTR_FarmTileState _tilestate))
  (switch string (Utilities|Array|Get(acopy) (LocalVariables|GettileStates) (Variables|Default|GetDEV%20state%20Counter))
    (:Till
      (Actions|TillTile))
    (:Water
      (Actions|WaterTile))
    (:Plant
      (Actions|PlantSeed "Carrot"))
    (:Grow1
      (Utilities|Map|Add _intvals "GrowthStage" 2)
      (CallFunction|InitGraphics :!label _label))
    (:Grow2
      (Utilities|Map|Add _intvals "GrowthStage" 3)
      (goto _label)))
  (Math|Integer|IncrementInt (Variables|Default|GetDEV%20state%20Counter)))