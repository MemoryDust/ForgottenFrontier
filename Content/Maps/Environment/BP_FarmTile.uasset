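; BP_FarmTile is a farm tile actor that exposes snap targets on its four sides.
; On BeginPlay, InitSnapTargets adds the west, east, north and south snap references to the SnapTargets array.
; The tile only builds this list; it contains no snapping logic, and its construction script is empty.
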(event EventBeginPlay
  (CallFunction|InitSnapTargets))

(event Collision|EventActorBeginOverlap
  (params (OtherActor :type Actor%20Object%20Reference)))

(event EventTick
  (params (DeltaSeconds :type Float%20%28single-precision%29)))

(fn ConstructionScript)

(fn InitSnapTargets
  (Utilities|Array|Add (Variables|Default|GetsnapTargets) (Variables|Default|GetWestSnap))
  (Utilities|Array|Add (Variables|Default|GetsnapTargets) (Variables|Default|GetEastSnap))
  (Utilities|Array|Add (Variables|Default|GetsnapTargets) (Variables|Default|GetNorthSnap))
  (Utilities|Array|Add (Variables|Default|GetsnapTargets) (Variables|Default|GetSouthSnap)))