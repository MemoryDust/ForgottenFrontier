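; BP_Prop is a configurable environment prop actor that displays a chosen static mesh with a chosen texture.
; The construction script assigns SetMesh to PropMesh, then builds a dynamic instance of the AlphaClipTextured_MAT material.
; It feeds SetTexture into that instance's Texture parameter and applies it to the mesh's first material slot.
; All setup happens at construction, with no active event graph logic.
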(event EventBeginPlay)

(event Collision|EventActorBeginOverlap
  (params (OtherActor :type Actor%20Object%20Reference)))

(event EventTick
  (params (DeltaSeconds :type Float%20%28single-precision%29)))

(fn ConstructionScript
  (CallFunction|InitMesh)
  (CallFunction|InitMaterials))

(fn InitMesh
  (Components|StaticMesh|SetStaticMesh (Variables|Default|GetPropMesh) (Variables|Default|GetSetMesh)))

(fn InitMaterials
  (bind _returnvalue (Rendering|Material|CreateDynamicMaterialInstance "/Game/Materials/AlphaClipTextured_MAT.AlphaClipTextured_MAT" "None" "None" :!class /Script/Engine.KismetMaterialLibrary))
  (bind _output_get (LocalVariables|SetdynaMat _returnvalue))
  (Rendering|Material|SetTextureParameterValue _output_get "Texture" (Variables|Default|GetSetTexture))
  (Rendering|Material|SetMaterial (Variables|Default|GetPropMesh) 0 (LocalVariables|GetdynaMat)))