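; Player farmer character for the overworld, handling camera-relative movement, dash and sprint, lock-on, item pickup and befriending Figments with held items.
; Lock-on searches tight, loose and nebulous volumes for "LookAt" actors, then steers control yaw toward the target.
; InteractionRadius feeds delayed pickup sweeps, the current spawn field and item giving, reporting to game instance, game mode and GUI.
; Dynamic materials texture face, body and the socket-following held item.
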(event OnComponentBeginOverlap(InteractionRadius)
  (params (OverlappedComponent :type Primitive%20Component%20Object%20Reference) (OtherActor :type Actor%20Object%20Reference) (OtherComp :type Primitive%20Component%20Object%20Reference) (OtherBodyIndex :type Integer) (bFromSweep :type Boolean) (SweepResult :type Hit%20Result%20Structure%20%28by%20ref%29))
  (bind _asfld_spawn_field (Utilities|Casting|CastToFLD_SpawnField OtherActor))
  (Variables|Default|SetcurrentSpawnField _asfld_spawn_field))

(event OnComponentEndOverlap(InteractionRadius)
  (params (OverlappedComponent :type Primitive%20Component%20Object%20Reference) (OtherActor :type Actor%20Object%20Reference) (OtherComp :type Primitive%20Component%20Object%20Reference) (OtherBodyIndex :type Integer))
  (Utilities|Casting|CastToFLD_SpawnField OtherActor)
  (Variables|Default|SetcurrentSpawnField 0))

(event OnComponentActivated(InteractionRadius)
  (params (Component :type Actor%20Component%20Object%20Reference) (bReset :type Boolean)))

(event EventBeginPlay
  (Init|InitGraphics)
  (Init|InitRefs)
  (CallFunction|SpawnonGround)
  (Utilities|FlowControl|Delay 1.0)
  (CallFunction|InitialSpawnFieldCheck))

(event Collision|EventActorBeginOverlap
  (params (OtherActor :type Actor%20Object%20Reference)))

(event EventTick
  (params (DeltaSeconds :type Float%20%28single-precision%29))
  (TickUpdate|AdjustRotationforLockon)
  (TickUpdate|UpdateSocketPositions)
  (Utilities|FlowControl|Delay 0.2)
  (if (not (.Targeting (Utilities|Struct|BreakSTR_AnimBools (Variables|Default|GetanimBools))))
    (Detection|SweepforInteractables)))

(event Input|ActionEvents|InputActionTarget
  (params (Key :type Key%20Structure :default "None"))
  (:Pressed
    (Utilities|Struct|SetmembersinSTR_AnimBools (Variables|Default|GetanimBools) true)
    (Variables|/Script/Engine.CharacterMovementComponent|SetbOrientRotationToMovement (Variables|Character|GetCharacterMovement) false)
    (Detection|FindLockonTarget))
  (:Released
    (Utilities|Struct|SetmembersinSTR_AnimBools (Variables|Default|GetanimBools) false)
    (Variables|/Script/Engine.CharacterMovementComponent|SetbOrientRotationToMovement (Variables|Character|GetCharacterMovement) true)
    (Variables|Default|SetbUseControllerRotationYaw false)
    (PlayerState|EndLockon)))

(event Input|ActionEvents|InputActionPutAway
  (params (Key :type Key%20Structure :default "None"))
  (:Pressed
    (if (.HoldingItem (Utilities|Struct|BreakSTR_AnimBools (Variables|Default|GetanimBools)))
      (CallFunction|PutAwayItem))))

(event Input|ActionEvents|InputActionConfirmButton
  (params (Key :type Key%20Structure :default "None"))
  (:Pressed
    (if (Variables|/Game/System/PC_Player.PC_Player_C|GetselectingItem? (Variables|KeyRefs|GetPC))
      (bind _holdsuccess_ (CallFunction|TryHoldItem))
      (if _holdsuccess_
        (Default|ToggleItemSelection (Variables|KeyRefs|GetPC)))
      (elif (.HoldingItem (Utilities|Struct|BreakSTR_AnimBools (Variables|Default|GetanimBools)))
        (CallFunction|TryGiveItem)
        (Default|RefreshItemsList (Variables|/Game/System/PC_Player.PC_Player_C|GetOverworldGUI (Variables|KeyRefs|GetPC)))
        (elif (Utilities|IsValid (Variables|Default|GetpickupActor))
          (Default|CollectItem (Variables|KeyRefs|GetGameInstance) (Variables|/Game/Actors/Items/BP_Item.BP_Item_C|GetitemName (Variables|Default|GetpickupActor)))
          (Default|ReceiveItemDespawnReport (Variables|KeyRefs|GetGameMode) (Variables|Default|GetpickupActor))
          (Variables|Default|SetpickupActor 0)
          (Variables|Default|SetfocusedActor 0)
          (Default|ToggleItemPickupPrompt (Variables|/Game/System/PC_Player.PC_Player_C|GetOverworldGUI (Variables|KeyRefs|GetPC)) false))))))

(event Input|ActionEvents|InputActionSprint
  (params (Key :type Key%20Structure :default "None"))
  (bind _animbools (Variables|Default|GetanimBools))
  (bind (_sprinting _dashing) (Utilities|Struct|BreakSTR_AnimBools _animbools))
  (:Pressed
    (Variables|Default|SetholdingSprint? true)
    (if (or (not _sprinting) (not _dashing))
      (Utilities|Struct|SetmembersinSTR_AnimBools (Variables|Default|GetanimBools) true)
      (Variables|/Script/Engine.CharacterMovementComponent|SetMaxWalkSpeed (Variables|Character|GetCharacterMovement) (Variables|Default|GetdashSpeed))
      (Variables|/Script/Engine.CharacterMovementComponent|SetMaxAcceleration (Variables|Character|GetCharacterMovement) 5e+03)))
  (:Released
    (Variables|Default|SetholdingSprint? false)
    (if (.Sprinting (Utilities|Struct|BreakSTR_AnimBools (Variables|Default|GetanimBools)))
      (Utilities|Struct|SetmembersinSTR_AnimBools (Variables|Default|GetanimBools) false false)
      (Variables|/Script/Engine.CharacterMovementComponent|SetMaxWalkSpeed (Variables|Character|GetCharacterMovement) (Variables|Default|GetwalkSpeed))
      (Variables|/Script/Engine.CharacterMovementComponent|SetMaxAcceleration (Variables|Character|GetCharacterMovement) 1.6e+03))))

(event Input|ActionEvents|InputActionItemSelectorMenu
  (params (Key :type Key%20Structure :default "None"))
  (:Pressed
    (Default|ToggleItemSelection (Variables|KeyRefs|GetPC))))

(event Input|AxisEvents|InputAxisMouseX
  (params (AxisValue :type Float%20%28single-precision%29))
  (Pawn|Input|AddControllerYawInput AxisValue))

(event Input|AxisEvents|InputAxisMouseY
  (params (AxisValue :type Float%20%28single-precision%29))
  (Pawn|Input|AddControllerPitchInput AxisValue))

(event Input|AxisEvents|InputAxisMoveForward
  (params (AxisValue :type Float%20%28single-precision%29))
  (Pawn|Input|AddMovementInput (Math|Vector|GetForwardVector (Math|Rotator|MakeRotator 0.0 0.0 (.Yaw (Math|Rotator|BreakRotator (Pawn|GetControlRotation :!class /Script/Engine.Pawn))))) AxisValue false)
  (if true
    _))

(event Input|AxisEvents|InputAxisMoveRight
  (params (AxisValue :type Float%20%28single-precision%29))
  (Pawn|Input|AddMovementInput (Math|Vector|GetRightVector (Math|Rotator|MakeRotator 0.0 0.0 (.Yaw (Math|Rotator|BreakRotator (Pawn|GetControlRotation :!class /Script/Engine.Pawn))))) AxisValue false)
  (if true
    _))

(fn ConstructionScript
  (Init|InitGraphics))

(fn FindLockonTarget
  (bind _targetfound_ (Detection|SweepforTargetables))
  (Utilities|Struct|SetmembersinSTR_AnimBools (Variables|Default|GetanimBools) _targetfound_)
  (Variables|Default|SetbUseControllerRotationYaw true))

(fn SweepforInteractables
  (bind _array_element (Utilities|Array|ForEachLoopwithBreak (Collision|GetOverlappingActors (Variables|Default|GetInteractionRadius) 0 :!class /Script/Engine.PrimitiveComponent) :!label _label)
    (:LoopBody
      (if (Actor|ActorHasTag _array_element "LookAt")
        (LocalVariables|SetfoundTarget true)
        (if (Actor|ActorHasTag _array_element "PickUp")
          (bind _asbp_item (Utilities|Casting|CastToBP_Item _array_element))
          (Variables|Default|SetpickupActor _asbp_item)
          (LocalVariables|SetfoundItem true)
          (goto _label Break))))
    (:Completed
      (if (LocalVariables|GetfoundTarget)
        (if (not (Variables|/Game/System/PC_Player.PC_Player_C|GetselectingItem? (Variables|KeyRefs|GetPC)))
          (if (LocalVariables|GetfoundItem)
            (Default|ToggleItemPickupPrompt (Variables|/Game/System/PC_Player.PC_Player_C|GetOverworldGUI (Variables|KeyRefs|GetPC)) true)
            (return true true)
            (else
              (Default|ToggleItemPickupPrompt (Variables|/Game/System/PC_Player.PC_Player_C|GetOverworldGUI (Variables|KeyRefs|GetPC)) false)
              (Variables|Default|SetpickupActor 0)
              (return true false))))
        (else
          (Variables|Default|SetfocusedActor 0)
          (Variables|Default|SetpickupActor 0)
          (Default|ToggleItemPickupPrompt (Variables|/Game/System/PC_Player.PC_Player_C|GetOverworldGUI (Variables|KeyRefs|GetPC)) false)
          (return false false))))))

(fn SweepforTargetables
  (bind _array_element (Utilities|Array|ForEachLoopwithBreak (Collision|GetOverlappingActors (Variables|Default|GetLockOnAreaTight) 0 :!class /Script/Engine.PrimitiveComponent) :!label _label)
    (:LoopBody
      (bind _output_get (LocalVariables|SettargetActor _array_element))
      (if (Actor|ActorHasTag _output_get "LookAt")
        (LocalVariables|SetfoundTarget true)
        (goto _label Break)))
    (:Completed
      (if (LocalVariables|GetfoundTarget)
        (Variables|Default|SetfocusedActor (LocalVariables|GettargetActor))
        (return true)
        (else
          (bind _array_element_2 (Utilities|Array|ForEachLoopwithBreak (Collision|GetOverlappingActors (Variables|Default|GetLockOnAreaLoose) 0 :!class /Script/Engine.PrimitiveComponent) :!label _label_2)
            (:LoopBody
              (bind _output_get_2 (LocalVariables|SettargetActor _array_element_2))
              (if (Actor|ActorHasTag _output_get_2 "LookAt")
                (LocalVariables|SetfoundTarget true)
                (goto _label_2 Break)))
            (:Completed
              (if (LocalVariables|GetfoundTarget)
                (Variables|Default|SetfocusedActor (LocalVariables|GettargetActor))
                (return true)
                (else
                  (bind _array_element_3 (Utilities|Array|ForEachLoopwithBreak (Collision|GetOverlappingActors (Variables|Default|GetLockOnAreaNebulous) 0 :!class /Script/Engine.PrimitiveComponent) :!label _label_3)
                    (:LoopBody
                      (bind _output_get_3 (LocalVariables|SettargetActor _array_element_3))
                      (if (Actor|ActorHasTag _output_get_3 "LookAt")
                        (goto _label_3 Break)))
                    (:Completed
                      (if (LocalVariables|GetfoundTarget)
                        (Variables|Default|SetfocusedActor (LocalVariables|GettargetActor))
                        (return true)
                        (else
                          (return false))))))))))))))

(fn InitRefs
  (bind _aspc_player (Utilities|Casting|CastToPC_Player (Game|GetPlayerController 0)))
  (Variables|KeyRefs|SetPC _aspc_player)
  (bind _asgi_forgotten_frontier (Utilities|Casting|CastToGI_ForgottenFrontier (Game|GetGameInstance)))
  (Variables|KeyRefs|SetGameInstance _asgi_forgotten_frontier)
  (bind _asgm_overworld (Utilities|Casting|CastToGM_Overworld (Game|GetGameMode)))
  (Variables|KeyRefs|SetGameMode _asgm_overworld))

(fn InitGraphics
  (bind _returnvalue (Rendering|Material|CreateDynamicMaterialInstance "/Game/Materials/AlphaClipTextured_MAT.AlphaClipTextured_MAT" "None" "None" :!class /Script/Engine.KismetMaterialLibrary))
  (bind _output_get (LocalVariables|SetFaceDyna _returnvalue))
  (Rendering|Material|SetTextureParameterValue _output_get "Texture" "/Game/Actors/Farmers/FarmerNEW/Textures/FarmerF_FaceRest_TEX.FarmerF_FaceRest_TEX")
  (Rendering|Material|SetMaterialbyName (Variables|Character|GetMesh) "Face" (LocalVariables|GetFaceDyna))
  (bind _returnvalue_2 (Rendering|Material|CreateDynamicMaterialInstance "/Game/Materials/AlphaClipTextured_MAT.AlphaClipTextured_MAT" "None" "None" :!class /Script/Engine.KismetMaterialLibrary))
  (bind _output_get_2 (LocalVariables|SetBodyDyna _returnvalue_2))
  (Rendering|Material|SetTextureParameterValue _output_get_2 "Texture" "/Game/Actors/Farmers/FarmerNEW/Textures/FarmerF_Body.FarmerF_Body")
  (Rendering|Material|SetMaterialbyName (Variables|Character|GetMesh) "Body" (LocalVariables|GetBodyDyna)))

(fn UpdateSocketPositions
  (bind _helditem (Variables|Default|GetHeldItem))
  (bind _mesh (Variables|Character|GetMesh))
  (bind _returnvalue (Transformation|GetSocketTransform _mesh "SOCK_HeldItem" "RTS_World"))
  (bind (_location _rotation) (Math|Transform|BreakTransform _returnvalue))
  (if (.HoldingItem (Utilities|Struct|BreakSTR_AnimBools (Variables|Default|GetanimBools)))
    (Transformation|SetWorldTransform _helditem (Math|Transform|MakeTransform _location _rotation (Transformation|GetWorldScale _helditem)) false false)))

(fn AdjustRotationforLockon
  (bind _returnvalue (Transformation|GetActorRotation))
  (if (.LockedOn (Utilities|Struct|BreakSTR_AnimBools (Variables|Default|GetanimBools)))
    (Pawn|SetControlRotation (Game|GetPlayerController 0) (Math|Rotator|MakeRotator (.roll _returnvalue) (.pitch _returnvalue) (.yaw (Math|Rotator|FindLookatRotation (Transformation|GetActorLocation) (Transformation|GetActorLocation (Variables|Default|GetfocusedActor))))))))

(fn CanControlCamera?
  (return (not false)))

(fn EndLockon
  (Utilities|Struct|SetmembersinSTR_AnimBools (Variables|Default|GetanimBools) false))

(fn TryRecallFigment)

(fn TryHoldItem
  (bind _outhelditem (Default|GetHeldItem (Variables|KeyRefs|GetPC)))
  (bind _output_get (LocalVariables|SetheldItemName _outhelditem))
  (if (Utilities|Enum|Equal(Enum) _output_get "")
    (return false)
    (else
      (Utilities|FlowControl|Sequence
        (:then_0
          (Utilities|Struct|SetmembersinSTR_AnimBools (Variables|Default|GetanimBools) true))
        (:then_1
          (bind (_outmodel _outtexture) (Default|LookupItemAesthetics (Variables|KeyRefs|GetGameInstance) (LocalVariables|GetheldItemName)))
          (LocalVariables|SetmeshTexture (.Value (Utilities|Map|Find _outtexture "Texture")))
          (Components|StaticMesh|SetStaticMesh (Variables|Default|GetHeldItem) _outmodel))
        (:then_2
          (bind _returnvalue (Rendering|Material|CreateDynamicMaterialInstance "/Game/Materials/AlphaClipTextured_MAT.AlphaClipTextured_MAT" "None" "None" :!class /Script/Engine.KismetMaterialLibrary))
          (LocalVariables|SetitemDynaMat _returnvalue)
          (Rendering|Material|SetTextureParameterValue (LocalVariables|GetitemDynaMat) "Texture" (LocalVariables|GetmeshTexture))
          (Rendering|Material|SetMaterial (Variables|Default|GetHeldItem) 0 (LocalVariables|GetitemDynaMat))
          (return true))))))

(fn PutAwayItem
  (Utilities|Struct|SetmembersinSTR_AnimBools (Variables|Default|GetanimBools) false)
  (Components|StaticMesh|SetStaticMesh (Variables|Default|GetHeldItem) 0))

(fn TryGiveItem
  (bind _outhelditem (Default|GetHeldItem (Variables|KeyRefs|GetPC)))
  (LocalVariables|SetheldItemName _outhelditem)
  (bind _asbp_figment (Utilities|Casting|CastToBP_Figment (Utilities|Array|Get(acopy) (Collision|GetOverlappingActors (Variables|Default|GetInteractionRadius) "/Game/Actors/Figments/Generic/BP_Figment.BP_Figment_C" :!class /Script/Engine.PrimitiveComponent))))
  (CallFunction|PutAwayItem)
  (bind _befriendsuccess_ (Default|TryBefriendFigment (Variables|KeyRefs|GetGameInstance) (Variables|/Game/Actors/Figments/Generic/BP_Figment.BP_Figment_C|GetoverworldID _asbp_figment) (LocalVariables|GetheldItemName)))
  (if _befriendsuccess_
    (Default|ReceiveFigmentDespawnReport (Variables|KeyRefs|GetGameMode) _asbp_figment)))

(fn InitialSpawnFieldCheck
  (bind _asfld_spawn_field (Utilities|Casting|CastToFLD_SpawnField (Utilities|Array|Get(acopy) (Collision|GetOverlappingActors (Variables|Default|GetInteractionRadius) "/Game/Maps/Fields/FLD_SpawnField.FLD_SpawnField_C" :!class /Script/Engine.PrimitiveComponent))))
  (Variables|Default|SetcurrentSpawnField _asfld_spawn_field))

(fn TryBeginSprint
  (if (Variables|Default|GetholdingSprint?)
    (Utilities|Struct|SetmembersinSTR_AnimBools (Variables|Default|GetanimBools) true false)
    (Variables|/Script/Engine.CharacterMovementComponent|SetMaxWalkSpeed (Variables|Character|GetCharacterMovement) (Variables|Default|GetsprintSpeed))
    (else
      (Utilities|Struct|SetmembersinSTR_AnimBools (Variables|Default|GetanimBools) false false)
      (Variables|/Script/Engine.CharacterMovementComponent|SetMaxWalkSpeed (Variables|Character|GetCharacterMovement) (Variables|Default|GetwalkSpeed))
      (Variables|/Script/Engine.CharacterMovementComponent|SetMaxAcceleration (Variables|Character|GetCharacterMovement) 1.6e+03))))

(fn SpawnonGround
  (bind _capsulecomponent (Variables|Collision|GetCapsuleComponent))
  (bind _returnvalue (Transformation|GetWorldLocation _capsulecomponent))
  (bind (_x _y) (Class|KismetMathLibrary|BreakVector3f _returnvalue))
  (bind (_x_2 _y_2 _z) (Class|KismetMathLibrary|BreakVector3f _returnvalue))
  (bind _outhit (Collision|LineTraceByChannel _returnvalue (Math|Vector|MakeVector _x_2 _y_2 (- _z 5e+02)) "TraceTypeQuery1" false 0 "None"))
  (if (Actor|ActorHasTag (.HitActor (Collision|BreakHitResult _outhit)) "Ground")
    (Transformation|SetActorLocation (Math|Vector|MakeVector _x _y (+ (.Z (Class|KismetMathLibrary|BreakVector3f (.ImpactPoint (Collision|BreakHitResult _outhit)))) (Variables|/Script/Engine.CapsuleComponent|GetCapsuleHalfHeight (Variables|Collision|GetCapsuleComponent)))) false false)))