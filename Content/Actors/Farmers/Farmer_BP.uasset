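; Farmer player character for an overworld game, with camera-relative movement, target lock-on and a capsule launcher for catching Figments.
; Targeting searches tiered overlap areas for "LookAt" actors, then turns control yaw toward the focus; otherwise Tick scans nearby interactables.
; Launcher input sets AnimBools flags; FireCapsule attempts capture through the game instance, reporting successful despawns to the game mode.
; It also tracks the current spawn field and creates face and equipment materials.
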(event OnComponentBeginOverlap(InteractionRadius)
  (params (OverlappedComponent :type Primitive%20Component%20Object%20Reference) (OtherActor :type Actor%20Object%20Reference) (OtherComp :type Primitive%20Component%20Object%20Reference) (OtherBodyIndex :type Integer) (bFromSweep :type Boolean) (SweepResult :type Hit%20Result%20Structure%20%28by%20ref%29))
  (bind _asfld_spawn_field (Utilities|Casting|CastToFLD_SpawnField OtherActor))
  (bind _output_get (Variables|Default|SetcurrentSpawnField _asfld_spawn_field))
  (Development|PrintString (Utilities|String|Append "Now entering " (Variables|/Game/Maps/Fields/FLD_SpawnField.FLD_SpawnField_C|GetFieldName _output_get))))

(event OnComponentEndOverlap(InteractionRadius)
  (params (OverlappedComponent :type Primitive%20Component%20Object%20Reference) (OtherActor :type Actor%20Object%20Reference) (OtherComp :type Primitive%20Component%20Object%20Reference) (OtherBodyIndex :type Integer))
  (bind _asfld_spawn_field (Utilities|Casting|CastToFLD_SpawnField OtherActor))
  (Variables|Default|SetcurrentSpawnField 0)
  (Development|PrintString (Utilities|String|Append "Now leaving  " (Variables|/Game/Maps/Fields/FLD_SpawnField.FLD_SpawnField_C|GetFieldName _asfld_spawn_field))))

(event Custom|CapsuleLaunchCooldown
  (Utilities|FlowControl|Delay 0.5)
  (Utilities|Struct|SetmembersinSTR_AnimBools (Variables|Default|GetanimBools) true))

(event EventBeginPlay
  (CallFunction|InitGraphics))

(event Collision|EventActorBeginOverlap
  (params (OtherActor :type Actor%20Object%20Reference)))

(event EventTick
  (params (DeltaSeconds :type Float%20%28single-precision%29))
  (CallFunction|AdjustRotationforLockon)
  (Utilities|FlowControl|Delay 0.2)
  (if (not (.Targeting (Utilities|Struct|BreakSTR_AnimBools (Variables|Default|GetanimBools))))
    (CallFunction|SweepforInteractables)))

(event Input|ActionEvents|InputActionTarget
  (params (Key :type Key%20Structure :default "None"))
  (:Pressed
    (Utilities|Struct|SetmembersinSTR_AnimBools (Variables|Default|GetanimBools) true)
    (Variables|/Script/Engine.CharacterMovementComponent|SetbOrientRotationToMovement (Variables|Character|GetCharacterMovement) false)
    (CallFunction|FindLockonTarget))
  (:Released
    (Utilities|Struct|SetmembersinSTR_AnimBools (Variables|Default|GetanimBools) false)
    (Variables|/Script/Engine.CharacterMovementComponent|SetbOrientRotationToMovement (Variables|Character|GetCharacterMovement) true)
    (Variables|Default|SetbUseControllerRotationYaw false)
    (CallFunction|EndLockon)))

(event Input|ActionEvents|InputActionCapsuleLauncher
  (params (Key :type Key%20Structure :default "None"))
  (bind _animbools (Variables|Default|GetanimBools))
  (bind (_lockedon _canfirecapsulelauncher) (Utilities|Struct|BreakSTR_AnimBools _animbools))
  (:Pressed
    (if (and _lockedon _canfirecapsulelauncher)
      (Utilities|Struct|SetmembersinSTR_AnimBools (Variables|Default|GetanimBools) true))))

(event Input|AxisEvents|InputAxisMouseX
  (params (AxisValue :type Float%20%28single-precision%29))
  (bind _cancontrolcamera_ (CallFunction|CanControlCamera?))
  (if _cancontrolcamera_
    (Pawn|Input|AddControllerYawInput AxisValue)))

(event Input|AxisEvents|InputAxisMouseY
  (params (AxisValue :type Float%20%28single-precision%29))
  (bind _cancontrolcamera_ (CallFunction|CanControlCamera?))
  (if _cancontrolcamera_
    (Pawn|Input|AddControllerPitchInput AxisValue)))

(event Input|AxisEvents|InputAxisMoveForward
  (params (AxisValue :type Float%20%28single-precision%29))
  (Pawn|Input|AddMovementInput (Math|Vector|GetForwardVector (Math|Rotator|MakeRotator 0.0 0.0 (.Yaw (Math|Rotator|BreakRotator (Pawn|GetControlRotation :!class /Script/Engine.Pawn))))) AxisValue false))

(event Input|AxisEvents|InputAxisMoveRight
  (params (AxisValue :type Float%20%28single-precision%29))
  (Pawn|Input|AddMovementInput (Math|Vector|GetRightVector (Math|Rotator|MakeRotator 0.0 0.0 (.Yaw (Math|Rotator|BreakRotator (Pawn|GetControlRotation :!class /Script/Engine.Pawn))))) AxisValue false))

(fn ConstructionScript
  (CallFunction|InitGraphics))

(fn InitGraphics
  (bind _returnvalue (Rendering|Material|CreateDynamicMaterialInstance "/Game/Materials/Solid_MAT.Solid_MAT" "None" "None" :!class /Script/Engine.KismetMaterialLibrary))
  (bind _output_get (LocalVariables|SetFaceDyna _returnvalue))
  (Rendering|Material|SetTextureParameterValue _output_get "Texture" "/Game/Actors/Farmers/Female/TEX/FarmerF_FaceRest_TEX.FarmerF_FaceRest_TEX")
  (Rendering|Material|SetMaterialbyName (Variables|Character|GetMesh) "Face" (LocalVariables|GetFaceDyna))
  (bind _returnvalue_2 (Rendering|Material|CreateDynamicMaterialInstance "/Game/Materials/Solid_MAT.Solid_MAT" "None" "None" :!class /Script/Engine.KismetMaterialLibrary))
  (bind _output_get_2 (LocalVariables|SetEquipmentDyna _returnvalue_2))
  (Rendering|Material|SetTextureParameterValue _output_get_2 "Texture" "/Game/Actors/Items/Gear/Swords/TEX_Tools.TEX_Tools")
  (Rendering|Material|SetMaterial (Variables|Default|GetEquipment) 0 _output_get_2))

(fn CanControlCamera?
  (return (not false)))

(fn FindLockonTarget
  (bind _targetfound_ (CallFunction|SweepforTargetables))
  (Utilities|Struct|SetmembersinSTR_AnimBools (Variables|Default|GetanimBools) _targetfound_)
  (Variables|Default|SetbUseControllerRotationYaw true))

(fn SweepforInteractables
  (bind _array_element (Utilities|Array|ForEachLoopwithBreak (Collision|GetOverlappingActors (Variables|Default|GetInteractionRadius) 0 :!class /Script/Engine.PrimitiveComponent) :!label _label)
    (:LoopBody
      (bind _output_get (LocalVariables|SettargetActor _array_element))
      (if (Actor|ActorHasTag _output_get "LookAt")
        (LocalVariables|SetfoundTarget true)
        (goto _label Break)))
    (:Completed
      (if (LocalVariables|GetfoundTarget)
        (Variables|Default|SetfocusTarget (LocalVariables|GettargetActor))
        (return true)
        (else
          (Variables|Default|SetfocusTarget 0)
          (return false))))))

(fn SweepforTargetables
  (bind _array_element (Utilities|Array|ForEachLoopwithBreak (Collision|GetOverlappingActors (Variables|Default|GetLockOnAreaTight) 0 :!class /Script/Engine.PrimitiveComponent) :!label _label)
    (:LoopBody
      (bind _output_get (LocalVariables|SettargetActor _array_element))
      (if (Actor|ActorHasTag _output_get "LookAt")
        (LocalVariables|SetfoundTarget true)
        (goto _label Break)))
    (:Completed
      (if (LocalVariables|GetfoundTarget)
        (Variables|Default|SetfocusTarget (LocalVariables|GettargetActor))
        (return true)
        (else
          (bind _array_element_2 (Utilities|Array|ForEachLoopwithBreak (Collision|GetOverlappingActors (Variables|Default|GetLockOnAreaLoose) 0 :!class /Script/Engine.PrimitiveComponent) :!label _label_2)
            (:LoopBody
              (bind _output_get_2 (LocalVariables|SettargetActor _array_element_2))
              (if (Actor|ActorHasTag _output_get_2 "LookAt")
                (LocalVariables|SetfoundTarget true)
                (goto _label_2 Break)))
            (:Completed
              (if (LocalVariables|GetfoundTarget)
                (Variables|Default|SetfocusTarget (LocalVariables|GettargetActor))
                (return true)
                (else
                  (bind _array_element_3 (Utilities|Array|ForEachLoopwithBreak (Collision|GetOverlappingActors (Variables|Default|GetLockOnAreaNebulous) 0 :!class /Script/Engine.PrimitiveComponent) :!label _label_3)
                    (:LoopBody
                      (bind _output_get_3 (LocalVariables|SettargetActor _array_element_3))
                      (if (Actor|ActorHasTag _output_get_3 "LookAt")
                        (goto _label_3 Break)))
                    (:Completed
                      (if (LocalVariables|GetfoundTarget)
                        (Variables|Default|SetfocusTarget (LocalVariables|GettargetActor))
                        (return true)
                        (else
                          (return false))))))))))))))

(fn AdjustRotationforLockon
  (bind _returnvalue (Transformation|GetActorRotation))
  (if (.LockedOn (Utilities|Struct|BreakSTR_AnimBools (Variables|Default|GetanimBools)))
    (Pawn|SetControlRotation (Game|GetPlayerController 0) (Math|Rotator|MakeRotator (.roll _returnvalue) (.pitch _returnvalue) (.yaw (Math|Rotator|FindLookatRotation (Transformation|GetActorLocation) (Transformation|GetActorLocation (Variables|Default|GetfocusTarget))))))))

(fn FireCapsule
  (CallFunction|TryCatchTarget))

(fn EndLockon
  (Utilities|Struct|SetmembersinSTR_AnimBools (Variables|Default|GetanimBools) false))

(fn EndFire
  (Utilities|Struct|SetmembersinSTR_AnimBools (Variables|Default|GetanimBools) false))

(fn TryCatchTarget
  (bind _asbp_figment (Utilities|Casting|CastToBP_Figment (Variables|Default|GetfocusTarget)))
  (bind _output_get (LocalVariables|SetfigmentTarget _asbp_figment))
  (if (Utilities|IsValid _output_get)
    (bind _asgi_forgotten_frontier (Utilities|Casting|CastToGI_ForgottenFrontier (Game|GetGameInstance)))
    (bind _capturesuccess_ (Default|TryCaptureFigment _asgi_forgotten_frontier (Variables|/Game/Actors/Figments/Generic/BP_Figment.BP_Figment_C|GetoverworldID (LocalVariables|GetfigmentTarget))))
    (if _capturesuccess_
      (CallFunction|EndLockon)
      (bind _asgm_overworld (Utilities|Casting|CastToGM_Overworld (Game|GetGameMode)))
      (Default|ReceiveDespawnReport _asgm_overworld (LocalVariables|GetfigmentTarget))
      (Development|PrintString "Catch successful!")
      (CallFunction|CapsuleLaunchCooldown)
      (else
        (Development|PrintString "Catch failed...")
        (CallFunction|CapsuleLaunchCooldown)))))