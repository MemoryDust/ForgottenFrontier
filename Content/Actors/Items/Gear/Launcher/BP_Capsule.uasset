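; BP_Capsule is a thrown capsule item from the launcher gear, used to catch Figments.
; When its Cube overlaps an actor it ignores BP_Farmer, and on a BP_Figment starts a catch attempt for the Thrower if that Figment is catchable, then destroys itself.
; Other actors leave it intact, and it self-destructs after a fixed delay from BeginPlay.
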(event OnComponentBeginOverlap(Cube)
  (params (OverlappedComponent :type Primitive%20Component%20Object%20Reference) (OtherActor :type Actor%20Object%20Reference) (OtherComp :type Primitive%20Component%20Object%20Reference) (OtherBodyIndex :type Integer) (bFromSweep :type Boolean) (SweepResult :type Hit%20Result%20Structure%20%28by%20ref%29))
  (Utilities|Casting|CastToBP_Farmer OtherActor
    (:CastFailed
      (bind _asbp_figment (Utilities|Casting|CastToBP_Figment OtherActor))
      (if (Variables|/Game/Actors/Figments/Generic/BP_Figment.BP_Figment_C|Getcatchable? _asbp_figment)
        (Default|BeginCatchAttempt _asbp_figment (Variables|Default|Getthrower)))
      (CallFunction|DestroyCapsule))))

(event EventBeginPlay
  (Utilities|FlowControl|Delay 1e+01)
  (Actor|DestroyActor))

(event Collision|EventActorBeginOverlap
  (params (OtherActor :type Actor%20Object%20Reference)))

(event EventTick
  (params (DeltaSeconds :type Float%20%28single-precision%29)))

(fn ConstructionScript)

(fn DestroyCapsule
  (Actor|DestroyActor))