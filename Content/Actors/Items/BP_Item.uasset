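; BP_Item is a world item actor that shows an item's looks and rests on the ground beneath it.
; On BeginPlay it pulls mesh and texture from the game instance by ItemName, applying a dynamic alpha-clip material.
; A delayed Tick repeats a downward trace, snapping the actor above "Ground"-tagged surfaces or reporting it once to GM_Overworld for despawn.
; The farmer overlap check currently takes no action.
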(event EventBeginPlay
  (CallFunction|InitGraphics)
  (CallFunction|DetectGround))

(event Collision|EventActorBeginOverlap
  (params (OtherActor :type Actor%20Object%20Reference)))

(event EventTick
  (params (DeltaSeconds :type Float%20%28single-precision%29))
  (Utilities|FlowControl|Delay 0.5)
  (CallFunction|CheckActualization)
  (if (not (Variables|Default|GetpendingDestroy))
    (CallFunction|DetectGround)))

(fn ConstructionScript)

(fn InitGraphics
  (bind _asgi_forgotten_frontier (Utilities|Casting|CastToGI_ForgottenFrontier (Game|GetGameInstance)))
  (bind (_outmodel _outtexture) (Default|LookupItemAesthetics _asgi_forgotten_frontier (Variables|Default|GetitemName)))
  (Components|StaticMesh|SetStaticMesh (Variables|Default|GetItemMesh) _outmodel)
  (bind _returnvalue (Rendering|Material|CreateDynamicMaterialInstance "/Game/Materials/AlphaClipTextured_MAT.AlphaClipTextured_MAT" "None" "None" :!class /Script/Engine.KismetMaterialLibrary))
  (bind _output_get (LocalVariables|SetdynaMat _returnvalue))
  (Rendering|Material|SetTextureParameterValue _output_get "Texture" (.Value (Utilities|Map|Find _outtexture "Texture")))
  (Rendering|Material|SetMaterial (Variables|Default|GetItemMesh) 0 (LocalVariables|GetdynaMat)))

(fn CheckActualization
  (if (Utilities|IsValid (Utilities|Array|Get(acopy) (Collision|GetOverlappingActors (Variables|Default|GetCapsule) "/Game/Actors/Farmers/BP_Farmer.BP_Farmer_C" :!class /Script/Engine.PrimitiveComponent)))
    _))

(fn DetectGround
  (bind _returnvalue (Transformation|GetActorLocation))
  (bind _itemmesh (Variables|Default|GetItemMesh))
  (bind _returnvalue_2 (Transformation|GetWorldLocation _itemmesh))
  (bind (_x _y) (Math|Vector|BreakVector _returnvalue))
  (bind (_x_2 _y_2) (Math|Vector|BreakVector _returnvalue_2))
  (bind (_outhit _returnvalue_3) (Collision|LineTraceByChannel _returnvalue_2 (Math|Vector|MakeVector _x_2 _y_2 (- 0.0 5e+02)) "TraceTypeQuery1" false 0 "None"))
  (if _returnvalue_3
    (if (Components|ComponentHasTag (.HitComponent (Collision|BreakHitResult _outhit)) "Ground")
      (LocalVariables|SethitLoc (.Location (Collision|BreakHitResult _outhit)))
      (Transformation|SetActorLocation (Math|Vector|MakeVector _x _y (+ (.Z (Math|Vector|BreakVector (LocalVariables|GethitLoc))) (+ (Variables|/Script/Engine.CapsuleComponent|GetCapsuleHalfHeight (Variables|Default|GetCapsule)) (Variables|Default|GetshadowOffset)))) true false)
      (else
        (CallFunction|BeginDestroy :!label _label)))
    (else
      (goto _label))))

(fn BeginDestroy
  (if (not (Variables|Default|GetpendingDestroy))
    (bind _asgm_overworld (Utilities|Casting|CastToGM_Overworld (Game|GetGameMode)))
    (Default|ReceiveItemDespawnReport _asgm_overworld self)
    (Variables|Default|SetpendingDestroy true)))