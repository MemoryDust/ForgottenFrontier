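; BP_ScreenshotFigment is a display version of a Figment, likely for screenshots, with no active event logic.
; InitGraphics takes a Figment ID and looks up its overworld aesthetics through GI_ForgottenFrontier.
; InitModel sets and scales the skeletal mesh, but leaves the passed anim class unused.
; InitMaterials builds dynamic Face and Body materials from AlphaClip_MAT, switching to ALT_-prefixed textures for off-color variants.
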(event EventBeginPlay)

(event Collision|EventActorBeginOverlap
  (params (OtherActor :type Actor%20Object%20Reference)))

(event EventTick
  (params (DeltaSeconds :type Float%20%28single-precision%29)))

(fn ConstructionScript)

(fn InitGraphics
  (params (inFigmentID :type Integer))
  (Variables|Default|SetfigmentID inFigmentID)
  (bind _asgi_forgotten_frontier (Utilities|Casting|CastToGI_ForgottenFrontier (Game|GetGameInstance)))
  (bind (_stats _textures _models _animclass _altcolor_) (Default|LookupFigmentOverworldAesthetics _asgi_forgotten_frontier (Variables|Default|GetfigmentID)))
  (CallFunction|InitModel _models _stats _animclass)
  (CallFunction|InitMaterials _textures _altcolor_))

(fn InitMaterials
  (params (inTexture :type Map%20of%20Strings%20to%20Objects) (inAltColor :type Boolean))
  (if inAltColor
    (Development|PrintString "OFF-COLOR SPAWNED!!!!")
    (LocalVariables|SetaltAppend "ALT_"))
  (bind _returnvalue (Rendering|Material|CreateDynamicMaterialInstance "/Game/Materials/AlphaClip_MAT.AlphaClip_MAT" "None" "None" :!class /Script/Engine.KismetMaterialLibrary))
  (bind _output_get (LocalVariables|SetFaceDyna _returnvalue))
  (Rendering|Material|SetTextureParameterValue _output_get "Texture" (.Value (Utilities|Map|Find inTexture (Utilities|String|Append (LocalVariables|GetaltAppend) "Face"))))
  (Rendering|Material|SetMaterialbyName (Variables|Character|GetMesh) "Face" (LocalVariables|GetFaceDyna))
  (bind _returnvalue_2 (Rendering|Material|CreateDynamicMaterialInstance "/Game/Materials/AlphaClip_MAT.AlphaClip_MAT" "None" "None" :!class /Script/Engine.KismetMaterialLibrary))
  (bind _output_get_2 (LocalVariables|SetBodyDyna _returnvalue_2))
  (Rendering|Material|SetTextureParameterValue _output_get_2 "Texture" (.Value (Utilities|Map|Find inTexture (Utilities|String|Append (LocalVariables|GetaltAppend) "Body"))))
  (Rendering|Material|SetMaterialbyName (Variables|Character|GetMesh) "Body" (LocalVariables|GetBodyDyna)))

(fn InitModel
  (params (inModel :type Map%20of%20Strings%20to%20Objects) (inStats :type Map%20of%20Strings%20to%20Reals) (inAnimClass :type Anim%20Instance%20Class%20Reference))
  (Class|SkinnedMeshComponent|SetSkeletalMesh (Variables|Character|GetMesh) (.Value (Utilities|Map|Find inModel "Main")) true)
  (Transformation|SetWorldScale3D (Variables|Character|GetMesh) (* (Transformation|GetWorldScale (Variables|Character|GetMesh)) (.Value (Utilities|Map|Find inStats "sizeMultiplier")))))