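; Overworld Figment actor: a catchable creature whose model, animation and face/body materials, including alternate colors, come from a game instance lookup by ID.
; A delayed Tick check traces down to "Ground" to snap the actor, or only its shadow when airborne.
; Missing ground or no BP_Farmer overlap reports despawn to GM_Overworld, unless player-owned or immune.
; Catch attempts are resolved by the game instance; success also reports despawn.
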(event EventBeginPlay
  (CallFunction|InitGraphics)
  (CallFunction|DetectGround))

(event Collision|EventActorBeginOverlap
  (params (OtherActor :type Actor%20Object%20Reference)))

(event EventTick
  (params (DeltaSeconds :type Float%20%28single-precision%29))
  (Utilities|FlowControl|Delay 0.5)
  (CallFunction|CheckActualization)
  (if (not (Variables|Default|GetToBeDestroyed))
    (CallFunction|DetectGround)))

(fn ConstructionScript)

(fn InitGraphics
  (bind _asgi_forgotten_frontier (Utilities|Casting|CastToGI_ForgottenFrontier (Game|GetGameInstance)))
  (bind (_stats _textures _models _animclass _altcolor_) (Default|LookupFigmentOverworldAesthetics _asgi_forgotten_frontier (Variables|Default|GetoverworldID) (Variables|Default|GetplayerOwned?)))
  (CallFunction|InitModel _models _stats _animclass)
  (CallFunction|InitMaterials _textures _altcolor_))

(fn InitMaterials
  (params (inTexture :type Map%20of%20Strings%20to%20Objects) (inAltColor :type Boolean))
  (if inAltColor
    (Development|PrintString "OFF-COLOR SPAWNED!!!!")
    (LocalVariables|SetaltAppend "ALT_"))
  (bind _returnvalue (Rendering|Material|CreateDynamicMaterialInstance "/Game/Materials/AlphaClipTextured_MAT.AlphaClipTextured_MAT" "None" "None" :!class /Script/Engine.KismetMaterialLibrary))
  (bind _output_get (LocalVariables|SetFaceDyna _returnvalue))
  (Rendering|Material|SetTextureParameterValue _output_get "Texture" (.Value (Utilities|Map|Find inTexture (Utilities|String|Append (LocalVariables|GetaltAppend) "Face"))))
  (Rendering|Material|SetMaterialbyName (Variables|Character|GetMesh) "Face" (LocalVariables|GetFaceDyna))
  (bind _returnvalue_2 (Rendering|Material|CreateDynamicMaterialInstance "/Game/Materials/AlphaClipTextured_MAT.AlphaClipTextured_MAT" "None" "None" :!class /Script/Engine.KismetMaterialLibrary))
  (bind _output_get_2 (LocalVariables|SetBodyDyna _returnvalue_2))
  (Rendering|Material|SetTextureParameterValue _output_get_2 "Texture" (.Value (Utilities|Map|Find inTexture (Utilities|String|Append (LocalVariables|GetaltAppend) "Body"))))
  (Rendering|Material|SetMaterialbyName (Variables|Character|GetMesh) "Body" (LocalVariables|GetBodyDyna)))

(fn InitModel
  (params (inModel :type Map%20of%20Strings%20to%20Objects) (inStats :type Map%20of%20Strings%20to%20Reals) (inAnimClass :type Anim%20Instance%20Class%20Reference))
  (bind _mesh (Variables|Character|GetMesh))
  (Class|SkinnedMeshComponent|SetSkeletalMesh (Variables|Character|GetMesh) (.Value (Utilities|Map|Find inModel "Main")) true)
  (Transformation|SetWorldScale3D _mesh (* (Transformation|GetWorldScale (Variables|Character|GetMesh)) (.Value (Utilities|Map|Find inStats "sizeMultiplier"))))
  (Class|SkeletalMeshComponent|SetAnimClass _mesh inAnimClass))

(fn CheckActualization
  (if (not (Utilities|IsValid (Utilities|Array|Get(acopy) (Collision|GetOverlappingActors (Variables|Collision|GetCapsuleComponent) "/Game/Actors/Farmers/BP_Farmer.BP_Farmer_C" :!class /Script/Engine.PrimitiveComponent))))
    (CallFunction|StartDestroy)))

(fn BeginCatchAttempt
  (params (inThrower :type BP%20Farmer%20Object%20Reference))
  (bind _output_get (LocalVariables|Setthrower inThrower))
  (Default|EndLockon _output_get)
  (Variables|Default|Setcatchable? false)
  (bind _asgi_forgotten_frontier (Utilities|Casting|CastToGI_ForgottenFrontier (Game|GetGameInstance)))
  (bind _capturesuccess_ (Default|TryCaptureFigment _asgi_forgotten_frontier (Variables|Default|GetoverworldID)))
  (if _capturesuccess_
    (bind _asgm_overworld (Utilities|Casting|CastToGM_Overworld (Game|GetGameMode)))
    (Default|ReceiveFigmentDespawnReport _asgm_overworld self)
    (Development|PrintString "Catch successful!")
    (else
      (Development|PrintString "Catch failed...")
      (Variables|Default|Setcatchable? true))))

(fn DetectGround
  (bind _returnvalue (Transformation|GetActorLocation))
  (bind _mesh (Variables|Character|GetMesh))
  (bind _shadow (Variables|Default|GetShadow))
  (bind _returnvalue_2 (Transformation|GetWorldLocation _mesh))
  (bind (_x _y) (Math|Vector|BreakVector _returnvalue))
  (bind _returnvalue_3 (Transformation|GetWorldLocation _shadow))
  (bind (_x_2 _y_2) (Math|Vector|BreakVector _returnvalue_3))
  (bind (_x_3 _y_3 _z) (Math|Vector|BreakVector _returnvalue_2))
  (bind (_outhits _returnvalue_4) (Class|KismetSystemLibrary|LineTraceMultiforObjects _returnvalue_2 (Math|Vector|MakeVector _x_3 _y_3 (- _z 5e+02)) (Utilities|Array|MakeArray "ObjectTypeQuery1") false 0 "None" true))
  (if _returnvalue_4
    (if (Actor|ActorHasTag (.HitActor (Collision|BreakHitResult (Utilities|Array|Get(acopy) _outhits))) "Ground")
      (LocalVariables|SethitLoc (.Location (Collision|BreakHitResult (Utilities|Array|Get(acopy) _outhits))))
      (if (Variables|Default|GetisAirborne)
        (Transformation|SetWorldLocation (Variables|Default|GetShadow) (Math|Vector|MakeVector _x_2 _y_2 (+ (.Z (Math|Vector|BreakVector (LocalVariables|GethitLoc))) (Variables|Default|GetshadowOffset))) true false)
        (else
          (Transformation|SetActorLocation (Math|Vector|MakeVector _x _y (+ (.Z (Math|Vector|BreakVector (LocalVariables|GethitLoc))) (+ (Variables|/Script/Engine.CapsuleComponent|GetCapsuleHalfHeight (Variables|Collision|GetCapsuleComponent)) (Variables|Default|GetshadowOffset)))) true false)))
      (else
        (CallFunction|StartDestroy :!label _label)))
    (else
      (goto _label))))

(fn StartDestroy
  (if (not (or (Variables|Default|GetplayerOwned?) (Variables|Default|GetimmuneToDestruction)))
    (bind _asgm_overworld (Utilities|Casting|CastToGM_Overworld (Game|GetGameMode)))
    (Default|ReceiveFigmentDespawnReport _asgm_overworld self)
    (Variables|Default|SetToBeDestroyed true)
    (Development|PrintString "Destroy I guess")))