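; PC_Player is the player controller, which sets up the player's on-screen UI and handles a spawn-clearing input.
; On BeginPlay, InitGUI creates the figment collection and overworld widgets, stores references to both and adds them to the viewport.
; Pressing the ClearSpawns action casts the game mode to GM_Overworld and calls its ClearSpawns function.
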(event EventBeginPlay
  (CallFunction|InitGUI))

(event EventTick
  (params (DeltaSeconds :type Float%20%28single-precision%29)))

(event Input|ActionEvents|InputActionClearSpawns
  (params (Key :type Key%20Structure :default "None"))
  (:Pressed
    (bind _asgm_overworld (Utilities|Casting|CastToGM_Overworld (Game|GetGameMode)))
    (Default|ClearSpawns _asgm_overworld)))

(fn ConstructionScript)

(fn InitGUI
  (bind _returnvalue (UserInterface|CreateWidget "/Game/UI/GUI_FigmentCollection.GUI_FigmentCollection_C"))
  (bind _output_get (Variables|Default|SetOwnedFigmentDisplay _returnvalue))
  (UserInterface|Viewport|AddtoViewport _output_get 0)
  (bind _returnvalue_2 (UserInterface|CreateWidget "/Game/UI/GUI_Overworld.GUI_Overworld_C"))
  (bind _output_get_2 (Variables|Default|SetOverworldGUI _returnvalue_2))
  (UserInterface|Viewport|AddtoViewport _output_get_2 0))