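; Overworld game mode that spawns and possesses the player's farmer and manages Figment and item actors around it.
; Tick uses delays to periodically top up wild Figments and items to their caps through the farmer's current spawn field, bounded by its spawn area.
; Despawn reports and send-out or recall functions keep actor lists updated, syncing Figment state to the game instance.
; BeginBattle is an empty stub.
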(event EventBeginPlay
  (CallFunction|DEV)
  (CallFunction|InitRefs))

(event EventTick
  (params (DeltaSeconds :type Float%20%28single-precision%29))
  ;[1 1 1] Fix this, it's ugly
  (bind _inaspawnfield_ (CallFunction|FindSpawnField))
  (if _inaspawnfield_
    (Utilities|FlowControl|Sequence
      (:then_0
        (Utilities|FlowControl|Delay 0.5)
        (bind (_inaspawnfield__2 _currentspawnfield) (CallFunction|FindSpawnField))
        (if _inaspawnfield__2
          (CallFunction|HandleFigmentSpawns _currentspawnfield)))
      (:then_1
        (Utilities|FlowControl|Delay 2.0)
        (bind (_inaspawnfield__3 _currentspawnfield_2) (CallFunction|FindSpawnField))
        (if _inaspawnfield__3
          (CallFunction|HandleItemSpawns _currentspawnfield_2))))))

(fn ConstructionScript)

(fn InitRefs
  (bind _farmerinst (Variables|Default|GetFarmerInst))
  (bind _aspc_player (Utilities|Casting|CastToPC_Player (Game|GetPlayerController 0)))
  (bind _output_get (LocalVariables|SetPC _aspc_player))
  (Pawn|Possess _output_get _farmerinst)
  (Variables|/Game/System/PC_Player.PC_Player_C|SetcontrolledCharacter (LocalVariables|GetPC) _farmerinst)
  (bind _asgi_forgotten_frontier (Utilities|Casting|CastToGI_ForgottenFrontier (Game|GetGameInstance)))
  (Variables|Default|SetGameInstance _asgi_forgotten_frontier))

(fn DEV
  (bind _returnvalue (Game|SpawnActorfromClass "/Game/Actors/Farmers/BP_Farmer.BP_Farmer_C" (Math|Transform|MakeTransform "0, 0,50.000000") "Undefined" 0 0))
  (Variables|Default|SetFarmerInst _returnvalue))

(fn HandleFigmentSpawns
  (params (currentSpawnField :type FLD%20Spawn%20Field%20Object%20Reference))
  (bind _activewildfigments (Variables|Default|GetactiveWildFigments))
  (bind _maxfigmentspawns (Variables|Default|GetmaxFigmentSpawns))
  (bind _returnvalue (Utilities|Array|Length _activewildfigments))
  (if (< _returnvalue _maxfigmentspawns)
    (bind _outfigmentsspawned (Default|SpawnFigments currentSpawnField (- _maxfigmentspawns _returnvalue) (Variables|/Game/Actors/Farmers/BP_Farmer.BP_Farmer_C|GetSpawnArea (Variables|Default|GetFarmerInst))))
    (for _array_element _outfigmentsspawned
      (Utilities|Array|Add (Variables|Default|GetactiveWildFigments) _array_element))))

(fn HandleItemSpawns
  (params (currentSpawnField :type FLD%20Spawn%20Field%20Object%20Reference))
  (bind _activeitems (Variables|Default|GetactiveItems))
  (bind _maxitemspawns (Variables|Default|GetmaxItemSpawns))
  (bind _returnvalue (Utilities|Array|Length _activeitems))
  (if (< _returnvalue _maxitemspawns)
    (bind _outspawneditems (Default|TrySpawnItems currentSpawnField (- _maxitemspawns _returnvalue) (Variables|/Game/Actors/Farmers/BP_Farmer.BP_Farmer_C|GetSpawnArea (Variables|Default|GetFarmerInst))))
    (for _array_element _outspawneditems
      (Utilities|Array|Add (Variables|Default|GetactiveItems) _array_element))))

(fn ClearSpawns
  (bind _activewildfigments (Variables|Default|GetactiveWildFigments))
  (bind _activeitems (Variables|Default|GetactiveItems))
  (Actor|DestroyActor _activewildfigments)
  (Utilities|Array|Clear _activewildfigments)
  (Actor|DestroyActor _activeitems)
  (Utilities|Array|Clear _activeitems))

(fn ReceiveFigmentDespawnReport
  (params (fromFigment :type BP%20Figment%20Object%20Reference))
  (Default|DespawnFigment (Variables|Default|GetGameInstance) (Variables|/Game/Actors/Figments/Generic/BP_Figment.BP_Figment_C|GetoverworldID fromFigment))
  (Utilities|Array|RemoveItem (Variables|Default|GetactiveWildFigments) fromFigment)
  (Actor|DestroyActor fromFigment))

(fn ReceiveItemDespawnReport
  (params (fromItem :type BP%20Item%20Object%20Reference))
  (Utilities|Array|RemoveItem (Variables|Default|GetactiveItems) fromItem)
  (Actor|DestroyActor fromItem))

(fn FindSpawnField
  (bind _farmerinst (Variables|Default|GetFarmerInst))
  (bind _currentspawnfield (Variables|/Game/Actors/Farmers/BP_Farmer.BP_Farmer_C|GetcurrentSpawnField _farmerinst))
  (return (Utilities|IsValid _currentspawnfield) _currentspawnfield))

(fn BeginBattle
  (params (playerFigmentID :type Integer) (wildFigmentID :type Integer)))

(fn RecallPlayerFigment
  (params (inFigmentID :type Integer))
  (Utilities|FlowControl|Sequence
    (:then_0
      (Default|SetSelectedFigmentIsOut (Variables|Default|GetGameInstance) inFigmentID false)
      (CallFunction|DespawnPlayerFigmentbyID inFigmentID))
    (:then_1
      (bind _aspc_player (Utilities|Casting|CastToPC_Player (Game|GetPlayerController 0))))))

(fn SendOutPlayerFigment
  (params (inFigmentID :type Integer) (inGeneralLocation :type Vector))
  (bind _returnvalue (Game|SpawnActorfromClass "/Game/Actors/Figments/Generic/BP_Figment.BP_Figment_C" (Math|Transform|MakeTransform inGeneralLocation) "Undefined" 0 inFigmentID true 0))
  (Utilities|Array|Add (Variables|Default|GetactivePlayerFigments) _returnvalue)
  (Default|SetSelectedFigmentIsOut (Variables|Default|GetGameInstance) inFigmentID true)
  (bind _aspc_player (Utilities|Casting|CastToPC_Player (Game|GetPlayerController 0))))

(fn DespawnPlayerFigmentbyID
  (params (inID :type Integer))
  (bind _array_element (Utilities|Array|ForEachLoopwithBreak (Variables|Default|GetactivePlayerFigments) :!label _label)
    (:LoopBody
      (if (== inID (Variables|/Game/Actors/Figments/Generic/BP_Figment.BP_Figment_C|GetoverworldID _array_element))
        (Actor|DestroyActor _array_element)
        (Utilities|Array|RemoveItem (Variables|Default|GetactivePlayerFigments) _array_element)
        (goto _label Break)))))